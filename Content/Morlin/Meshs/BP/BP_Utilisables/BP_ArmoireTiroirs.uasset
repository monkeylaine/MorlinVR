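; BP_ArmoireTiroirs is a usable drawer cabinet prop whose drawer slides on a physics constraint.
; On BeginPlay, it offsets the constraint's Frame1 reference from the drawer's position along the constraint's local X by DrawerLinearLimit.
; It then limits linear X travel to that same value, so the drawer's starting position sits at one end of the sliding range.
; Only Drawer1 is set up in the graph.
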(event EventBeginPlay
  ;[1 1 1] Begin Play - set physics constraint reference position and linear x limit
  (Class|PhysicsConstraintComponent|SetConstraintReferencePosition (Variables|Default|GetDrawer1Constraint) "Frame1" (+ (Transformation|GetWorldLocation (Variables|Default|GetDrawer1)) (Math|Transform|TransformDirection (Transformation|GetWorldTransform (Variables|Default|GetDrawer1Constraint)) (Math|Vector|MakeVector (Variables|Default|GetDrawerLinearLimit) 0.0 0.0))))
  (Class|PhysicsConstraintComponent|SetLinearXLimit (Variables|Default|GetDrawer1Constraint) "LCM_Limited" (Variables|Default|GetDrawerLinearLimit)))

(fn ConstructionScript)