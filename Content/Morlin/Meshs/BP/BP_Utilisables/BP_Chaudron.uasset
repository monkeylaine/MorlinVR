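; BP_Chaudron is a cauldron with a hinged door that triggers cooking and a recipe attempt when shut.
; Tick polls Door1's relative roll, using separate open and close thresholds to toggle IsOpen.
; Opening spawns a bubble effect below the arrow if none exists and prints its name.
; Closing calls CallCookPrimary on the SteamVR_GM game mode, destroys the bubbles, then runs CallRecetteTry.
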(event EventTick
  (params (DeltaSeconds :type Float%20%28single-precision%29))
  (if (Variables|Default|GetIsOpen)
    (if (> (.roll (Variables|/Script/Engine.SceneComponent|GetRelativeRotation (Variables|Default|GetDoor1))) -0.5)
      (Variables|Default|SetIsOpen false)
      (bind _assteam_vr_gm (Utilities|Casting|CastToSteamVR_GM (Game|GetGameMode)))
      (Default|CallCookPrimary _assteam_vr_gm)
      (Rendering|SetVisibility (Variables|Default|GetBubble) false false)
      (Components|DestroyComponent (Variables|Default|GetBubble))
      (Default|CallRecetteTry))
    (elif (< (.roll (Variables|/Script/Engine.SceneComponent|GetRelativeRotation (Variables|Default|GetDoor1))) -5.0)
      (Variables|Default|SetIsOpen true)
      (Utilities|IsValid (Variables|Default|GetBubble)
        (:Is%20Not%20Valid
          (bind _returnvalue (Niagara|SpawnSystematLocation "/Game/Morlin/FX/Bubbles/FX_Bubbles.FX_Bubbles" (+ (Transformation|GetWorldLocation (Variables|Default|GetArrow)) "0, 0,-10.000000") "0, 0, 0" "1.000000,1.000000,1.000000" false))
          (Variables|Default|SetBubble _returnvalue)
          (Development|PrintString (Utilities|GetDisplayName _returnvalue)))))))

(fn ConstructionScript)