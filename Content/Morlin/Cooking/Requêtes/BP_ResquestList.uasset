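; BP_ResquestList is an actor in the cooking requests folder that turns to face the player.
; Every Tick, it sets its rotation with a look-at from its own location to player pawn 0's location.
; A timeline that would move and rotate it along a referenced Path spline is present but never runs.
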(event EventBeginPlay)

(event EventTick
  (params (DeltaSeconds :type Float%20%28single-precision%29))
  (Transformation|SetActorRotation (Math|Rotator|FindLookatRotation (Transformation|GetActorLocation) (Transformation|GetActorLocation (Game|Player|GetPlayerPawn 0)))))

(fn ConstructionScript)