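; Base physics-driven grippable ingredient for cooking, which can start hidden and without collision until unlocked.
; Hit plays a random handling sound, throttled by a DoOnce that is also reset after a startup delay.
; Touching BP_GroundCollision plays a drop sound; if still grounded after a delay, the ingredient returns to its starting transform with impact and poof effects.
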(event Custom|resetTransform
  (bind _origintransform (Variables|Default|GetoriginTransform))
  (Rendering|SetActorHiddenInGame false)
  (Transformation|SetWorldTransform (Variables|Components|GetStaticMesh) (Variables|Default|GetoriginTransform) false false)
  (Niagara|SpawnSystematLocation "/Game/Morlin/FX/Soline/FX_Poof.FX_Poof" (.location _origintransform) (.rotation _origintransform) (.scale _origintransform)))

(event Custom|unlockIngredient
  (bind _staticmesh (Variables|Components|GetStaticMesh))
  (Variables|Default|Setlock true)
  (Rendering|SetVisibility _staticmesh true true)
  (Collision|SetCollisionEnabled _staticmesh "QueryAndPhysics"))

(event Custom|ResetHit
  (Utilities|FlowControl|DoOnce true) ; enters at Reset
)

(event EventBeginPlay
  (bind _staticmesh (Variables|Components|GetStaticMesh))
  (Physics|SetSimulatePhysics (Variables|Components|GetStaticMesh) true)
  (Variables|Default|SetoriginTransform (Transformation|GetWorldTransform (Variables|Components|GetStaticMesh)))
  (Utilities|FlowControl|Sequence
    (:then_0
      (if (Variables|Default|Getlock)
        (Rendering|SetVisibility _staticmesh false true)
        (Collision|SetCollisionEnabled _staticmesh "NoCollision")))
    (:then_1
      (Utilities|FlowControl|Delay 4.0)
      (CallFunction|ResetHit))))

(event Collision|EventActorBeginOverlap
  (params (OtherActor :type Actor%20Object%20Reference))
  (bind _staticmesh (Variables|Components|GetStaticMesh))
  (bind _returnvalue (Transformation|GetWorldTransform _staticmesh))
  (Utilities|Casting|CastToBP_ParentIngredientGrippable self)
  (Utilities|Casting|CastToBP_GroundCollision OtherActor)
  (Variables|Default|SetonGround true)
  (Audio|PlaySound2D (Utilities|Select :Index (Math|Random|RandomIntegerinRange 0 4) :Option%200 "/Game/Morlin/Sounds/Interactions/ES_Magazine_Drop_1_-_SFX_Producer.ES_Magazine_Drop_1_-_SFX_Producer" :Option%201 "/Game/Morlin/Sounds/Interactions/ES_Textbook_Drop_1_-_SFX_Producer.ES_Textbook_Drop_1_-_SFX_Producer" :Option%202 "/Game/Morlin/Sounds/Interactions/ES_Textbook_Drop_3_-_SFX_Producer.ES_Textbook_Drop_3_-_SFX_Producer" :Option%203 "/Game/Morlin/Sounds/Spécifique/ObjectFalls.ObjectFalls") 1.0 1.0 0.0 0 0)
  (Utilities|FlowControl|Delay 3.0)
  (if (Variables|Default|GetonGround)
    (Niagara|SpawnSystematLocation "/Game/Morlin/FX/ImpactEffect/FX_ImpactEffect.FX_ImpactEffect" (.location _returnvalue) (.rotation _returnvalue) (.scale _returnvalue))
    (Utilities|FlowControl|Delay 0.05)
    (CallFunction|ResetTransform)))

(event EventTick
  (params (DeltaSeconds :type Float%20%28single-precision%29)))

(event Collision|EventActorEndOverlap
  (params (OtherActor :type Actor%20Object%20Reference))
  (Utilities|Casting|CastToBP_GroundCollision OtherActor)
  (Variables|Default|SetonGround false))

(event Collision|EventHit
  (params (MyComp :type Primitive%20Component%20Object%20Reference) (Other :type Actor%20Object%20Reference) (OtherComp :type Primitive%20Component%20Object%20Reference) (bSelfMoved :type Boolean) (HitLocation :type Vector :default "0, 0, 0") (HitNormal :type Vector :default "0, 0, 0") (NormalImpulse :type Vector :default "0, 0, 0") (Hit :type Hit%20Result%20Structure%20%28by%20ref%29))
  (Utilities|FlowControl|DoOnce true
    (:Completed
      (Audio|PlaySoundatLocation (Utilities|Select :Index (Math|Random|RandomIntegerinRange 0 2) :Option%200 "/Game/Morlin/Sounds/Spécifique/TakingObject.TakingObject" :Option%201 "/Game/Morlin/Sounds/Interactions/ES_Baseball_Glove_4_-_SFX_Producer.ES_Baseball_Glove_4_-_SFX_Producer" :Option%202 "/Game/Morlin/Sounds/Spécifique/ObjectFalls.ObjectFalls") (Transformation|GetWorldLocation (Variables|Components|GetStaticMesh)) "0, 0, 0" 1.0 1.0 0.0 0 0 0)
      (Utilities|FlowControl|Delay 0.5)
      (CallFunction|ResetHit))))

(fn ConstructionScript)