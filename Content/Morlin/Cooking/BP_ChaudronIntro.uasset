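; VR intro cauldron that turns dropped ingredients into potions and doubles as a menu, where start and exit potions load day one or quit.
; Overlapping ingredients are recorded by class and hidden, updating the game mode and left-page widget.
; CookPrimary resets those actors for reuse, then matches recipes by count and membership, spawning the result or a random failure with effects.
; Construction Script builds the tutorial or main recipe list.
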(event Custom|CookPrimary
  (bind _wbp_leftpageref (Variables|Default|GetWBP_LeftPageRef))
  (if (> (Utilities|Array|Length (Variables|Default|GetIngredients)) 1)
    (CallFunction|RespawnIngredients)
    ;[1 1 1] SOund cook
    (Audio|PlaySound2D "/Game/Morlin/Sounds/Interactions/ES_ErianneWin.ES_ErianneWin" 1.0 1.0 0.0 0 0)
    (for (_array_element _array_index) (Variables|Default|GetPrimaryRecipeList)
      (Variables|Default|SetCurrentRecipeIndex _array_index)
      (if (Utilities|CompareLength _array_element)
        (Variables|Default|SetRecipeList (.Ingredients (Utilities|Struct|BreakS_CraftPrimaire _array_element)))
        (Variables|Default|SetNumberOfIngredientCorresponding 0)
        (for _array_element_2 (Variables|Default|GetIngredients)
          (if (Utilities|Array|ContainsItem (Variables|Default|GetRecipeList) _array_element_2)
            (Math|Integer|IncrementInt (Variables|Default|GetNumberOfIngredientCorresponding))))
        (if (== (Variables|Default|GetNumberOfIngredientCorresponding) (Utilities|Array|Length (.Ingredients (Utilities|Struct|BreakS_CraftPrimaire (Utilities|Array|Get(acopy) (Variables|Default|GetPrimaryRecipeList) (Variables|Default|GetCurrentRecipeIndex))))))
          (Variables|Default|SetGoodRecipeIndex (Variables|Default|GetCurrentRecipeIndex))
          (Variables|Default|SetRecipeFound true))))
    (if (Variables|Default|GetRecipeFound)
      (Game|SpawnActorfromClass (.Result (Utilities|Struct|BreakS_CraftPrimaire (Utilities|Array|Get(acopy) (Variables|Default|GetPrimaryRecipeList) (Variables|Default|GetGoodRecipeIndex)))) (Utilities|SpawnPos) "AdjustIfPossibleButAlwaysSpawn" 0 0)
      (Niagara|SpawnSystemAttached "/Game/Morlin/FX/Morlin/NS_Win.NS_Win" (Variables|Default|GetSphere) "None" "0, 0,50.000000" "0, 0, 0" "SnapToTarget" true)
      (Audio|SpawnSound2D "/Game/Morlin/FX/Morlin/S_GoodResult.S_GoodResult" 1.0 1.0 0.0 0)
      (bind _assteam_vr_gm (Utilities|Casting|CastToSteamVR_GM (Game|GetGameMode)))
      (Default|ReturnCraftedResult _assteam_vr_gm (.Result (Utilities|Struct|BreakS_CraftPrimaire (Utilities|Array|Get(acopy) (Variables|Default|GetPrimaryRecipeList) (Variables|Default|GetGoodRecipeIndex)))))
      (Utilities|IsValid _wbp_leftpageref
        (:Is%20Valid
          (Default|ResetIngredientNbr _wbp_leftpageref))
        (:Is%20Not%20Valid
          _))
      (Utilities|ResetVar)
      (else
        (Game|SpawnActorfromClass (Utilities|GetRandomResult) (Utilities|SpawnPos) "Undefined" 0 0)
        (Niagara|SpawnSystemAttached "/Game/Morlin/FX/Morlin/NS_BadResult.NS_BadResult" (Variables|Default|GetSphere) "None" "0, 0,50.000000" "0, 0, 0" "SnapToTarget" true)
        (Niagara|SpawnSystematLocation "/Game/Morlin/FX/Morlin/NS_Degradation.NS_Degradation" "-159.000000,261.000000,423.000000")
        (Audio|PlaySound2D "/Game/Morlin/FX/Morlin/S_BadResult.S_BadResult" 1.0 1.0 0.0 0 0)
        (Audio|PlaySound2D "/Game/Morlin/Sounds/Interactions/ES_WoodBad.ES_WoodBad" 1.0 1.0 0.0 0 0)
        (Default|ResetIngredientNbr (Variables|Default|GetWBP_LeftPageRef))
        (Utilities|ResetVar)))))

(event Custom|GetLeftPageRef
  (params (NewParam :type WBP%20Book%20Right%20Page%20Object%20Reference))
  (Variables|Default|SetWBP_LeftPageRef NewParam))

(event Collision|EventActorBeginOverlap
  (params (OtherActor :type Actor%20Object%20Reference))
  ;[1 1 1] Comment
  (Utilities|Casting|CastToBP_PotionStart OtherActor
    (:then
      (Game|OpenLevel(byName) "MorlinMapJour1"))
    (:CastFailed
      (Utilities|Casting|CastToPotionEXIT OtherActor
        (:then
          (Game|QuitGame 0 "Quit" false))
        (:CastFailed
          (bind _asbp_parent_ingredient_grippable (Utilities|Casting|CastToBP_ParentIngredientGrippable OtherActor))
          (CallFunction|AddIngredient _asbp_parent_ingredient_grippable)
          (Default|CallIngrdientin)
          (Utilities|FlowControl|Delay 1.0))))))

(event EventTick
  (params (DeltaSeconds :type Float%20%28single-precision%29)))

(fn ConstructionScript
  (Game|GetCurrentLevelName true)
  (if (Variables|Default|Getistuto)
    ;[1 0.7639 0.1963 1 35] Recette TUTO
    (Utilities|Array|Add (Variables|Default|GetPrimaryRecipeList) (Utilities|Struct|MakeS_CraftPrimaire "/Game/Morlin/Cooking/Resultats/Relaxation.Relaxation_C" (Utilities|Array|MakeArray "/Game/Morlin/Cooking/Ingredients/BP_GrippableIngredients/Compote/BP_CompoteOeil.BP_CompoteOeil_C" "/Game/Morlin/Cooking/Ingredients/BP_GrippableIngredients/BP_Dent_De_Loup.BP_Dent_De_Loup_C" "/Game/Morlin/Cooking/Ingredients/BP_GrippableIngredients/Jus/BP_JusDeMenthe.BP_JusDeMenthe_C")))
    (else
      (Utilities|FlowControl|Sequence
        (:then_0
          ;[0.05708 0.3069 1] Craft primaire -> copier coller le tous pour chaque recette
          (Utilities|Array|Add (Variables|Default|GetPrimaryRecipeList) (Utilities|Struct|MakeS_CraftPrimaire "/Game/Morlin/Cooking/Resultats/Murgier.Murgier_C" (Utilities|Array|MakeArray "/Game/Morlin/Cooking/Ingredients/BP_GrippableIngredients/BP_Ecorce_Arbre.BP_Ecorce_Arbre_C" "/Game/Morlin/Cooking/Ingredients/BP_GrippableIngredients/BP_Eau_Du_Lac.BP_Eau_Du_Lac_C" "/Game/Morlin/Cooking/Ingredients/BP_GrippableIngredients/BP_Citron.BP_Citron_C" "/Game/Morlin/Cooking/Ingredients/BP_GrippableIngredients/Compote/BP_CompoteOeil.BP_CompoteOeil_C") "/Game/Morlin/Sounds/Sous-Titres/Commandes/DialogueMurgier.DialogueMurgier"))
          ;[0.05708 0.3069 1] Craft primaire -> copier coller le tous pour chaque recette
          (Utilities|Array|Add (Variables|Default|GetPrimaryRecipeList) (Utilities|Struct|MakeS_CraftPrimaire "/Game/Morlin/Cooking/Resultats/Coudebouste.Coudebouste_C" (Utilities|Array|MakeArray "/Game/Morlin/Cooking/Ingredients/BP_GrippableIngredients/BP_Draginine.BP_Draginine_C" "/Game/Morlin/Cooking/Ingredients/BP_GrippableIngredients/BP_Eau_Du_Lac.BP_Eau_Du_Lac_C" "/Game/Morlin/Cooking/Ingredients/BP_GrippableIngredients/Jus/BP_JusDeDents.BP_JusDeDents_C" "/Game/Morlin/Cooking/Ingredients/BP_GrippableIngredients/BP_Feuille_De_Menthe.BP_Feuille_De_Menthe_C") "/Game/Morlin/Sounds/Sous-Titres/Commandes/DialoguesCoudebouste.DialoguesCoudebouste"))
          ;[0.05708 0.3069 1] Craft primaire -> copier coller le tous pour chaque recette
          (Utilities|Array|Add (Variables|Default|GetPrimaryRecipeList) (Utilities|Struct|MakeS_CraftPrimaire "/Game/Morlin/Cooking/Resultats/Eaudodo.Eaudodo_C" (Utilities|Array|MakeArray "/Game/Morlin/Cooking/Ingredients/BP_GrippableIngredients/BP_Mucus_Serpent.BP_Mucus_Serpent_C" "/Game/Morlin/Cooking/Ingredients/BP_GrippableIngredients/BP_Sangsue.BP_Sangsue_C" "/Game/Morlin/Cooking/Ingredients/BP_GrippableIngredients/BP_Oeil.BP_Oeil_C") "/Game/Morlin/Sounds/Sous-Titres/Commandes/DialoguesEaudodo.DialoguesEaudodo"))
          ;[0.05708 0.3069 1] Craft primaire -> copier coller le tous pour chaque recette
          (Utilities|Array|Add (Variables|Default|GetPrimaryRecipeList) (Utilities|Struct|MakeS_CraftPrimaire "/Game/Morlin/Cooking/Resultats/Ecladent.Ecladent_C" (Utilities|Array|MakeArray "/Game/Morlin/Cooking/Ingredients/BP_GrippableIngredients/Compote/BP_CompoteOeil.BP_CompoteOeil_C" "/Game/Morlin/Cooking/Ingredients/BP_GrippableIngredients/BP_Dent_De_Loup.BP_Dent_De_Loup_C" "/Game/Morlin/Cooking/Ingredients/BP_GrippableIngredients/BP_Cendre_De_Mamie.BP_Cendre_De_Mamie_C") "/Game/Morlin/Sounds/Sous-Titres/Commandes/DialoguesEcladent.DialoguesEcladent")))
        (:then_1
          ;[1 0.1281 0] Craft secondaire -> copier coller le tous pour chaque recette
          (Utilities|Array|Add (Variables|Default|GetSecondaryRecipeList) (Utilities|Struct|MakeS_CraftSecondaire (Utilities|GetRandomResult) (Utilities|Array|MakeArray "/Game/Morlin/Cooking/BP_ParentIngredientGrippable.BP_ParentIngredientGrippable_C"))))))))

(fn AddIngredient
  (params (AddedIngredient :type BP%20Parent%20Ingredient%20Grippable%20Object%20Reference))
  (bind _soundingredientin (Variables|Default|GetSoundIngredientIn))
  (bind _wbp_leftpageref (Variables|Default|GetWBP_LeftPageRef))
  (Utilities|FlowControl|Sequence
    (:then_0
      (Utilities|Array|Add (Variables|Default|GetIngredients) (Utilities|GetClass AddedIngredient))
      (Niagara|SpawnSystemAttached "/Game/Morlin/FX/IngredientDestroy/IngredientDestroy_System.IngredientDestroy_System" (Variables|Default|GetSphere1) "None" "0, 0, 0" "0, 0, 0" "KeepRelativeOffset" true)
      (Rendering|SetActorHiddenInGame AddedIngredient true)
      (Utilities|Array|Add (Variables|Default|GetHiddenIngredients) AddedIngredient)
      (bind _assteam_vr_gm (Utilities|Casting|CastToSteamVR_GM (Game|GetGameMode)))
      (Default|UpdateIngredientList _assteam_vr_gm (Variables|Default|GetIngredients))
      (Utilities|IsValid _wbp_leftpageref
        (:Is%20Valid
          (Default|UpIngredientNbr _wbp_leftpageref)
          (return))))
    (:then_1
      (Audio|PlaySound2D (Utilities|Array|Get(acopy) _soundingredientin (Math|Random|RandomIntegerinRange 0 (- (Utilities|Array|Length _soundingredientin) 1))) 1.0 1.0 0.0 0 0))))

(fn RespawnIngredients
  (for _array_element (Variables|Default|GetHiddenIngredients)
    (Default|ResetTransform _array_element))
  (Utilities|Array|Clear (Variables|Default|GetHiddenIngredients)))