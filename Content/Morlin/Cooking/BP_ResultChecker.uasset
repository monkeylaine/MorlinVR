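; BP_ResultChecker is the delivery check of the VR potion-cooking game, where Erianne reacts to the result handed over.
; A box overlap compares the BP_Resultat's class to ResultNeeded.
; A match plays her good montage, sound and particles, destroys the item, then after a delay unlocks the next ingredient through SteamVR_GM and broadcasts ReceivedCorrectPotion.
; A wrong result plays her bad montage, gated by a DoOnce that resets when the montage length elapses.
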(event OnComponentBeginOverlap(Box)
  (params (OverlappedComponent :type Primitive%20Component%20Object%20Reference) (OtherActor :type Actor%20Object%20Reference) (OtherComp :type Primitive%20Component%20Object%20Reference) (OtherBodyIndex :type Integer) (bFromSweep :type Boolean) (SweepResult :type Hit%20Result%20Structure%20%28by%20ref%29))
  (bind _asbp_resultat (Utilities|Casting|CastToBP_Resultat OtherActor))
  (if (== (Utilities|GetClass _asbp_resultat) (Variables|Default|GetResultNeeded))
    (bind _asabp_erianne (Utilities|Casting|CastToABP_Erianne (Components|SkeletalMesh|GetAnimInstance (Variables|Default|GetSkeletalMesh))))
    (Animation|Montage|MontagePlay _asabp_erianne "/Game/Morlin/Animations/Erianne/A_GoodResult_Montage.A_GoodResult_Montage" 1.0 "MontageLength" 0.0 true)
    (Actor|DestroyActor OtherActor)
    (Audio|SpawnSound2D "/Game/Morlin/Sounds/Interactions/ES_ErianneWin.ES_ErianneWin" 1.0 1.0 0.0 0)
    (Effects|SpawnEmitteratLocation 0 "0, 0, 0" "0, 0, 0" "0.500000,0.500000,0.500000" true "AutoRelease")
    (Utilities|FlowControl|Delay 3.0)
    (bind _assteam_vr_gm (Utilities|Casting|CastToSteamVR_GM (Game|GetGameMode)))
    (Default|UnlockNextIngredient _assteam_vr_gm)
    (Default|CallReceivedCorrectPotion)
    (else
      (Utilities|FlowControl|DoOnce false :!label _label
        (:Completed
          (bind _asabp_erianne_2 (Utilities|Casting|CastToABP_Erianne (Components|SkeletalMesh|GetAnimInstance (Variables|Default|GetSkeletalMesh))))
          (bind _returnvalue (Animation|Montage|MontagePlay _asabp_erianne_2 "/Game/Morlin/Animations/Erianne/A_BadResult_Montage.A_BadResult_Montage" 1.0 "MontageLength" 0.0 true))
          (Utilities|FlowControl|Delay _returnvalue)
          (goto _label Reset))))))

(event EventBeginPlay)

(event EventTick
  (params (DeltaSeconds :type Float%20%28single-precision%29)))

(fn ConstructionScript)