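; Base actor for cooking ingredients that can be locked and that return to their starting spot when dropped on the ground.
; Locked ingredients start hidden without collision until UnlockIngredient restores both.
; BeginPlay stores the mesh's world transform as the origin.
; Overlapping BP_GroundCollision plays a fall sound, then after a delay, if still grounded, teleports the mesh home with Niagara effects, except for BP_Resultat instances.
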(event Custom|UnlockIngredient
  (bind _staticmeshcomponent (Variables|Default|GetStaticMeshComponent))
  (Variables|Default|SetUnlock true)
  (Rendering|SetVisibility _staticmeshcomponent true false)
  (Collision|SetCollisionEnabled _staticmeshcomponent "QueryAndPhysics"))

(event Custom|ResetTransform
  (Transformation|SetWorldTransform (Variables|Default|GetStaticMeshComponent) (Variables|Default|GetOriginTransform) false true))

(event EventBeginPlay
  (bind _staticmeshcomponent (Variables|Default|GetStaticMeshComponent))
  (|CallParentFunction)
  (Variables|Default|SetOriginTransform (Transformation|GetWorldTransform (Variables|Default|GetStaticMeshComponent)))
  (if (not (Variables|Default|GetUnlock))
    (Rendering|SetVisibility _staticmeshcomponent false false)
    (Collision|SetCollisionEnabled _staticmeshcomponent "NoCollision")))

(event Collision|EventActorBeginOverlap
  (params (OtherActor :type Actor%20Object%20Reference))
  (bind _staticmeshcomponent (Variables|Default|GetStaticMeshComponent))
  (bind _origintransform (Variables|Default|GetOriginTransform))
  (bind _returnvalue (Transformation|GetWorldTransform _staticmeshcomponent))
  (Utilities|Casting|CastToBP_Resultat self
    (:CastFailed
      (Utilities|Casting|CastToBP_GroundCollision OtherActor)
      (Variables|Default|SetOnGround true)
      (Audio|PlaySound2D "/Game/Morlin/Sounds/Spécifique/ObjectFalls.ObjectFalls" 1.0 1.0 0.0 0 0)
      (Utilities|FlowControl|Delay 5.0)
      (if (Variables|Default|GetOnGround)
        (Niagara|SpawnSystematLocation "/Game/Morlin/FX/ImpactEffect/FX_ImpactEffect.FX_ImpactEffect" (.location _returnvalue) (.rotation _returnvalue) (.scale _returnvalue))
        (Utilities|FlowControl|Delay 0.05)
        (CallFunction|ResetTransform)
        (Niagara|SpawnSystematLocation "/Game/Morlin/FX/Soline/FX_Poof.FX_Poof" (.location _origintransform) (.rotation _origintransform) (.scale _origintransform))))))

(event Collision|EventActorEndOverlap
  (params (OtherActor :type Actor%20Object%20Reference))
  (Utilities|Casting|CastToBP_GroundCollision OtherActor)
  (Variables|Default|SetOnGround false))

(fn ConstructionScript
  (|CallParentFunction))