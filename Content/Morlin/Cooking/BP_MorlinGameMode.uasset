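; Game mode for Morlin's cooking gameplay, acting as a relay between the cauldron (BP_Chaudron) and the UI widget.
; It caches the first cauldron found at BeginPlay and receives the widget reference through GetUIRef.
; Ingredient list updates are stored here, with only the item count passed on to the UI.
; CallCookPrimary forwards the cook request to the cauldron's CookPrimary.
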(event Custom|GetUIRef
  (params (WBP_UI :type WBP%20UI%20Object%20Reference))
  (Variables|Default|SetWBP_UI_Ref WBP_UI))

(event Custom|UpdateIngredientList
  (params (IngredientList :type Array%20of%20S%20Object%20Info%20Structures))
  (bind _output_get (Variables|Default|SetIngredientList IngredientList))
  (Default|UpdateIngredientList (Variables|Default|GetWBP_UI_Ref) (Utilities|Array|Length _output_get)))

(event Custom|CallCookPrimary
  (Default|CookPrimary (Variables|Default|GetChaudronRef)))

(event EventBeginPlay
  (bind _outactors (Actor|GetAllActorsOfClass "/Game/Morlin/Cooking/BP_Chaudron.BP_Chaudron_C"))
  (Variables|Default|SetChaudronRef (Utilities|Array|Get(acopy) _outactors)))

(fn ConstructionScript)