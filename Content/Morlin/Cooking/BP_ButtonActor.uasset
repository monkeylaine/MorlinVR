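; BP_ButtonActor is a button actor for the cooking system that triggers primary cooking through the SteamVR_GM game mode.
; Its button component's state-change event calls CallCookPrimary when on and sets the text render to Off when off.
; BeginPlay also shows the Off text if the button starts off.
; Logic for signalling electrical targets and a CallButtonPressed call are present but unconnected.
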(event OnButtonStateChanged(ButtonComp)
  (params (ButtonState :type Boolean) (InteractingActor :type Actor%20Object%20Reference) (InteractingComponent :type Primitive%20Component%20Object%20Reference))
  (bind _assteam_vr_gm (Utilities|Casting|CastToSteamVR_GM (Game|GetGameMode)))
  (if ButtonState
    (Default|CallCookPrimary _assteam_vr_gm)
    (else
      (Rendering|Components|TextRender|SetText (Variables|Components|GetTextRender) (Variables|Default|GetOff)))))

(event EventBeginPlay
  (if (not (Variables|/Script/VRExpansionPlugin.VRButtonComponent|GetbButtonState (Variables|Default|GetButtonComp)))
    (Rendering|Components|TextRender|SetText (Variables|Components|GetTextRender) (Variables|Default|GetOff))))

(event EventTick
  (params (DeltaSeconds :type Float%20%28single-precision%29)))

(fn ConstructionScript)