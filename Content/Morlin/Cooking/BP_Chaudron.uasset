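; VR cauldron that crafts potions from ingredients dropped into it, and also starts the level or quits when special menu potions touch it.
; Overlapping ingredients are stored, destroyed with an effect and reported to SteamVR_GM and the left-page widget.
; CookPrimary matches ingredient count and classes against construction-script recipes, spawning the result above the cauldron, or a random one on failure, then resets.
; Secondary recipes are populated, but their cooking logic is disconnected.
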(event Custom|CookPrimary
  (bind _wbp_leftpageref (Variables|Default|GetWBP_LeftPageRef))
  (if (< (Utilities|Array|Length (Variables|Default|GetIngredient)) 2)
    (Development|PrintString "You need at least 2 ingredients" true true "(R=1.000000,G=0.000000,B=0.000000,A=1.000000)" 5.0)
    (else
      (for (_array_element _array_index) (Variables|Default|GetPrimaryRecipeList)
        (Variables|Default|SetCurrentRecipeIndex _array_index)
        (if (Utilities|CompareLength _array_element)
          (for _array_element_2 (.Ingredients (Utilities|Struct|BreakS_CraftPrimaire _array_element))
            (Utilities|Array|Add (Variables|Default|GetRecipeList) _array_element_2))
          (for _array_element_3 (Variables|Default|GetIngredient)
            (if (Utilities|Array|ContainsItem (Variables|Default|GetRecipeList) (Utilities|GetClass _array_element_3))
              (Variables|Default|SetNumberOfIngredientCorresponding (+ (Variables|Default|GetNumberOfIngredientCorresponding) 1))))
          (if (== (Variables|Default|GetNumberOfIngredientCorresponding) (Utilities|Array|Length (.Ingredients (Utilities|Struct|BreakS_CraftPrimaire (Utilities|Array|Get(acopy) (Variables|Default|GetPrimaryRecipeList) (Variables|Default|GetCurrentRecipeIndex))))))
            (Variables|Default|SetGoodRecipeIndex (Variables|Default|GetCurrentRecipeIndex))
            (Variables|Default|SetRecipeFound true)
            (else
              (Variables|Default|SetNumberOfIngredientCorresponding 0)))))
      (if (Variables|Default|GetRecipeFound)
        (Game|SpawnActorfromClass (.Result (Utilities|Struct|BreakS_CraftPrimaire (Utilities|Array|Get(acopy) (Variables|Default|GetPrimaryRecipeList) (Variables|Default|GetGoodRecipeIndex)))) (Utilities|SpawnPos) "Undefined" 0 0)
        (bind _assteam_vr_gm (Utilities|Casting|CastToSteamVR_GM (Game|GetGameMode)))
        (Default|ReturnCraftedResult _assteam_vr_gm (.Result (Utilities|Struct|BreakS_CraftPrimaire (Utilities|Array|Get(acopy) (Variables|Default|GetPrimaryRecipeList) (Variables|Default|GetGoodRecipeIndex)))))
        (Audio|SpawnSoundatLocation "/Game/Morlin/Sounds/Spécifique/Win.Win" "0, 0, 0" "0, 0, 0" 1.0 1.0 0.0 0 0)
        (Utilities|IsValid _wbp_leftpageref
          (:Is%20Valid
            (Default|ResetIngredientNbr _wbp_leftpageref))
          (:Is%20Not%20Valid
            _))
        (Utilities|ResetVar)
        (else
          (Game|SpawnActorfromClass (Utilities|GetRandomResult) (Utilities|SpawnPos) "Undefined" 0 0)
          (Default|ResetIngredientNbr (Variables|Default|GetWBP_LeftPageRef))
          (Utilities|ResetVar))))))

(event Custom|GetLeftPageRef
  (params (NewParam :type WBP%20Book%20Right%20Page%20Object%20Reference))
  (Variables|Default|SetWBP_LeftPageRef NewParam))

(event Collision|EventActorBeginOverlap
  (params (OtherActor :type Actor%20Object%20Reference))
  (Utilities|Casting|CastToBP_PotionStart OtherActor
    (:then
      (Game|OpenLevel(byName) "MorlinMapJour1"))
    (:CastFailed
      (Utilities|Casting|CastToPotionEXIT OtherActor
        (:then
          (Game|QuitGame 0 "Quit" false))
        (:CastFailed
          (bind _asbp_parent_ingredient (Utilities|Casting|CastToBP_ParentIngredient OtherActor))
          (CallFunction|AddIngredient _asbp_parent_ingredient)
          (Default|CallIngrdientin))))))

(fn ConstructionScript
  (Utilities|FlowControl|Sequence
    (:then_0
      ;[0.05708 0.3069 1] Craft primaire -> copier coller le tous pour chaque recette
      (Utilities|Array|Add (Variables|Default|GetPrimaryRecipeList) (Utilities|Struct|MakeS_CraftPrimaire "/Game/Morlin/Cooking/Resultats/Recette_2.Recette_2_C" (Utilities|Array|MakeArray "/Game/Morlin/Cooking/Ingredients/BP_Jour_01/BP_CendresDeMamie.BP_CendresDeMamie_C" "/Game/Morlin/Cooking/Ingredients/BP_Jour_01/BP_BecDeCorbeau.BP_BecDeCorbeau_C" "/Game/Morlin/Cooking/Ingredients/BP_Jour_01/BP_GousseAil.BP_GousseAil_C"))))
    (:then_1
      ;[1 0.1281 0] Craft secondaire -> copier coller le tous pour chaque recette
      (Utilities|Array|Add (Variables|Default|GetSecondaryRecipeList) (Utilities|Struct|MakeS_CraftSecondaire (Utilities|GetRandomResult) (Utilities|Array|MakeArray "/Game/Morlin/Cooking/BP_ParentIngredient.BP_ParentIngredient_C"))))))

(fn AddIngredient
  (params (AddedIngredient :type BP%20Parent%20Ingredient%20Object%20Reference))
  (bind _wbp_leftpageref (Variables|Default|GetWBP_LeftPageRef))
  (Utilities|Array|Add (Variables|Default|GetIngredient) AddedIngredient)
  (Development|PrintString (Utilities|String|Append "L'ingrédient : " (Utilities|GetDisplayName AddedIngredient) " a été ajouter au chaudron."))
  (Niagara|SpawnSystemAttached "/Game/Morlin/FX/IngredientDestroy/IngredientDestroy_System.IngredientDestroy_System" (Variables|Default|GetSphere1) "None" "0, 0, 0" "0, 0, 0" "KeepRelativeOffset" true)
  (Actor|DestroyActor AddedIngredient)
  (bind _assteam_vr_gm (Utilities|Casting|CastToSteamVR_GM (Game|GetGameMode)))
  (Default|UpdateIngredientList _assteam_vr_gm (Variables|Default|GetIngredient))
  (Utilities|IsValid _wbp_leftpageref
    (:Is%20Valid
      (Default|UpIngredientNbr _wbp_leftpageref))))