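; VR jar actor (BocaleOeil, a cooking ingredient) with a removable stopper, built on the VR grip interface with gripping denied on the actor itself.
; Gripping the stopper detaches it and stores the controller, so overlapping the neck capsule makes that controller drop and socket it onto the potion mesh.
; Releasing the potion mesh force-checks overlaps (engine bug workaround) and attaches it, physics off, to any overlapping "Body" mesh as makeshift inventory.
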(event OnComponentBeginOverlap(NeckCapsule)
  (params (OverlappedComponent :type Primitive%20Component%20Object%20Reference) (OtherActor :type Actor%20Object%20Reference) (OtherComp :type Primitive%20Component%20Object%20Reference) (OtherBodyIndex :type Integer) (bFromSweep :type Boolean) (SweepResult :type Hit%20Result%20Structure%20%28by%20ref%29))
  ;[1 1 1] On Begin Overlap (Neck Capsule) - drop from controller and attach to the potion mesh
  (if (== OtherComp (Variables|Default|GetStopper)) ; Is the overlapping object the stopper mesh?
    (Utilities|IsValid (Variables|Default|GetStopperController)
      (:Is%20Valid
        (Class|GripMotionControllerComponent|DropandSocketObject (Variables|Default|GetStopperController) (Class|VRExpansionFunctionLibrary|MakeTransformNetQuantize "0, 0, 0" "0, 0, 0" "1,1,1") (Variables|Default|GetStopper) 0 (Variables|Default|GetPotionMesh) "None" true)))))

(event EventOnChildGrip
  (params (GrippingController :type Grip%20Motion%20Controller%20Component%20Object%20Reference) (GripInformation :type BP%20Actor%20Grip%20Information%20Structure%20%28by%20ref%29))
  (bind (_gripid _griptargettype _grippedobject) (Utilities|Struct|BreakBPActorGripInformation GripInformation))
  ;[1 1 1] On Child Grip (BPI call) -
  (switch Utilities|FlowControl|Switch|SwitchonEGripTargetType _griptargettype
    (:ComponentGrip
      (Utilities|IsValid _grippedobject
        (:Is%20Valid
          (if (== _grippedobject (Variables|Default|GetStopper)) ; Is the gripped object the stopper?
            (Variables|Default|SetStopperController GrippingController) ; Set player controller for later reference
            (Transformation|DetachFromComponent (Variables|Default|GetStopper) "KeepWorld" "KeepWorld" "KeepWorld" true) ; This is supposed to happen automatically, but it doesn't....
          ))))))

(event EventOnChildGripRelease
  (params (ReleasingController :type Grip%20Motion%20Controller%20Component%20Object%20Reference) (GripInformation :type BP%20Actor%20Grip%20Information%20Structure%20%28by%20ref%29) (bWasSocketed :type Boolean))
  (bind (_gripid _griptargettype _grippedobject) (Utilities|Struct|BreakBPActorGripInformation GripInformation))
  ;[1 1 1] On Child Grip Release (BPI call) - remove player controller as stopper controller
  (switch Utilities|FlowControl|Switch|SwitchonEGripTargetType _griptargettype
    (:ComponentGrip
      (Utilities|IsValid _grippedobject
        (:Is%20Valid
          (if (== _grippedobject (Variables|Default|GetStopper)) ; Is the stopper the girpped object?
            (Variables|Default|SetStopperController 0) ; Set controller to none, it was the last player controller that gripped it
            (else
              ;[1 1 1] After grip release, Attach to inventory (player "Body" mesh) if overlapping - just a hackish example
              (if (== _grippedobject (Variables|Default|GetPotionMesh)) ; Is the gripped object the potion mesh?
                (bind _outcomponents (Class|KismetSystemLibrary|ComponentOverlapComponents (Variables|Default|GetPotionMesh) (Transformation|GetWorldTransform (Variables|Default|GetPotionMesh)) (Utilities|Array|MakeArray "ObjectTypeQuery3") "/Script/Engine.StaticMeshComponent" (Utilities|Array|MakeArray self))) ; Force checking overlaps due to engine bug
                (bind _array_element (Utilities|Array|ForEachLoopwithBreak _outcomponents :!label _label)
                  (:LoopBody
                    (if (Utilities|Enum|Equal(Enum) (Utilities|GetObjectName _array_element) "Body") ; Is the overlapped component the Body of the VR player character?
                      (Physics|SetSimulatePhysics (Variables|Default|GetPotionMesh) false) ; Stop simulating the potion mesh
                      (Transformation|AttachComponentToComponent (Variables|Default|GetPotionMesh) _array_element "None" "KeepWorld" "KeepWorld" "KeepWorld" true) ; Attach the potion mesh to the VR player
                      (goto _label Break))))))))))))

(fn ConstructionScript)

(fn AdvancedGripSettings
  (return ""))

(fn AllowsMultipleGrips
  (return false))

(fn ClosestGripSlotinRange
  (params (WorldLocation :type Vector :default "0, 0, 0") (bSecondarySlot :type Boolean) (CallingController :type Grip%20Motion%20Controller%20Component%20Object%20Reference) (OverridePrefix :type Name :default "None"))
  (return false "" "None"))

(fn DenyGripping
  (params (GripInitiator :type Grip%20Motion%20Controller%20Component%20Object%20Reference))
  (return true))

(fn GetGripScripts
  (return 0 false))

(fn GetGripStiffnessandDamping
  (return 0.0 0.0))

(fn GetPrimaryGripType
  (params (bIsSlot :type Boolean))
  (return "InteractiveCollisionWithPhysics"))

(fn GripBreakDistance
  (return 0.0))

(fn GripLateUpdateSetting
  (return "LateUpdatesAlwaysOn"))

(fn GripMovementReplicationType
  (return "KeepOriginalMovement"))

(fn IsHeld
  (return 0 false))

(fn RequestsSocketing
  (return 0 "None" "" false))

(fn SecondaryGripType
  (return "SG_None"))

(fn SimulateonDrop
  (return false))

(fn TeleportBehavior
  (return "TeleportAllComponents"))