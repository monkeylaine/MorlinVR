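; BP_Resultat_Child is a child Blueprint among the cooking ingredients, apparently a cooking result object.
; On BeginPlay it runs the parent logic, then makes its StaticMesh visible and turns on physics simulation for it.
; All other behavior comes from the parent class, as its overlap and tick events are disabled stubs and its construction script only calls the parent.
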(event EventBeginPlay
  (bind _staticmesh (Variables|Default|GetStaticMesh))
  (|CallParentFunction)
  (Rendering|SetVisibility _staticmesh true false)
  (Development|SetHiddeninGame _staticmesh false false)
  (Physics|SetSimulatePhysics _staticmesh true))

(event Collision|EventActorBeginOverlap
  (params (OtherActor :type Actor%20Object%20Reference))
  (|CallParentFunction OtherActor) ; This node is disabled and will not be called.\nDrag off pins to build functionality.
)

(event EventTick
  (params (DeltaSeconds :type Float%20%28single-precision%29))
  (|CallParentFunction DeltaSeconds) ; This node is disabled and will not be called.\nDrag off pins to build functionality.
)

(fn ConstructionScript
  (|CallParentFunction))